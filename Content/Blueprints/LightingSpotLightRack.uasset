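; Spotlight rack actor that gathers its eight spotlights into an array on BeginPlay.
; An unfinished rotation effect uses a timeline update to set each light's world rotation, interpolating from the actor's rotation toward a fresh random rotator with fixed delta time and speed.
; Nothing starts that timeline and Tick is empty, so this Blueprint does not move the lights at runtime.
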(event `self.ReceiveBeginPlay`
  (set `self.LightArray` (`|MakeArray` (`self.SpotLight1`) (`self.SpotLight2`) (`self.SpotLight3`) (`self.SpotLight4`) (`self.SpotLight5`) (`self.SpotLight6`) (`self.SpotLight7`) (`self.SpotLight`))))

(event `self.ReceiveTick`
  (params (DeltaSeconds :type "Float (single-precision)")))

(fn `UserConstructionScript`)