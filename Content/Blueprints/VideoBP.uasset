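; VideoBP is a video screen manager that registers screen actors in the level and starts playback of a test video.
; On BeginPlay it gathers actors tagged VideoScreen into an array and an index-keyed map, then opens the source on a media player.
; DetermineScreenArea runs for each screen but is only a stub that prints a debug string per array element when the index is found in the map.
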(event `self.ReceiveBeginPlay`
  (`|ExecutionSequence`
    (:`then_0`
      (bind _outactors (`GameplayStatics.GetAllActorsWithTag` "VideoScreen"))
      (bind _output_get (set `self.ScreenArray` _outactors))
      (for (_array_element _array_index) _output_get
        (`BlueprintMapLibrary.Map_Add` (`self.ScreenMap`) _array_index _array_element)
        (`self.DetermineScreenArea` _array_index)))
    (:`then_1`
      (`MediaPlayer.OpenSource` (`self.MediaPlayer`) "/Game/Materials/TestVideo.TestVideo"))))

(event `DetermineScreenArea`
  (params (ScreenIndex :type Integer))
  (for _ (`self.ScreenArray`)
    (if (`.ReturnValue` (`BlueprintMapLibrary.Map_Find` (`self.ScreenMap`) ScreenIndex))
      (`KismetSystemLibrary.PrintString` "Hello"))))

(fn `UserConstructionScript`)